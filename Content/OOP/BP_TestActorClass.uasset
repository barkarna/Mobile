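; BP_TestActorClass is a test actor in the OOP folder that holds an HP value with damage and healing functions.
; TakeDamage subtracts from HP and floors the result at zero.
; Heal adds to HP through a clamp that uses current HP as the minimum and a hardcoded maximum of 100.
; BeginPlay calls TakeDamage with zero damage, and Heal is not called within this Blueprint.
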(event `self.ReceiveBeginPlay`
  (`self.TakeDamage` 0))

(fn `Heal`
  (params (HPToAdd :type Integer))
  (bind _hp (`self.HP`))
  (set `self.HP` (`KismetMathLibrary.Clamp` (+ _hp HPToAdd) _hp 100)))

(fn `TakeDamage`
  (params (DamageValue :type Integer))
  (bind _returnvalue (- (`self.HP`) DamageValue))
  (if (> _returnvalue 0)
    (set `self.HP` _returnvalue)
    (else
      (set `self.HP` 0))))

(fn `UserConstructionScript`)